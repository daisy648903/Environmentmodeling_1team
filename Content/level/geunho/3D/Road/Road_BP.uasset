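; Spline-driven road actor that builds a deformed road with optional curbs in the construction script, with no runtime logic.
; It tiles spline mesh components by mesh length, clamping tangents to segment length.
; Curbs use right-vector and Z offsets, and Mirror adds the opposite side when Curbs is on.
; StartingCurbPosition returns a zero start position, leaving its offset calculation unconnected, so non-mirrored curb segments all start at the local origin.
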(fn `EndingCurbPosition`
  (params (CurbIndex :type Integer))
  (returns (EndingPositon :type "Vector Structure") (EndingTangent :type "Vector Structure"))
  (bind _spline (`self.Spline`))
  (bind _returnvalue (* (+ CurbIndex 1) (`self.CurbMeshLenth`)))
  (bind (_returnvalue_x _returnvalue_y _returnvalue_z) (`KismetMathLibrary.BreakVector` (+ (* (`SplineComponent.GetRightVectorAtDistanceAlongSpline` (`self.Spline`) _returnvalue "Local") (`self.CurbOffset`)) (`SplineComponent.GetLocationAtDistanceAlongSpline` _spline _returnvalue "Local"))))
  (return (`KismetMathLibrary.MakeVector` _returnvalue_x _returnvalue_y (+ _returnvalue_z (`self.ZOffset`))) (`KismetMathLibrary.ClampVectorSize` (`SplineComponent.GetTangentAtDistanceAlongSpline` _spline _returnvalue "Local") 0.0 (`self.CurbMeshLenth`))))

(fn `EndingRoadPosition`
  (params (RoadIndex :type Integer))
  (returns (EndingPositon :type "Vector Structure") (EndingTangent :type "Vector Structure"))
  (bind _spline (`self.Spline`))
  (bind _returnvalue (* (+ RoadIndex 1) (`self.RoadMeshLength`)))
  (return (`SplineComponent.GetLocationAtDistanceAlongSpline` _spline _returnvalue "Local") (`KismetMathLibrary.ClampVectorSize` (`SplineComponent.GetTangentAtDistanceAlongSpline` _spline _returnvalue "Local") 0.0 (`self.RoadMeshLength`))))

(fn `MirrorCurbPosionEnd`
  (params (CurbIndex :type Integer))
  (returns (EndingPositon :type "Vector Structure") (EndingTangent :type "Vector Structure"))
  (bind _spline (`self.Spline`))
  (bind _returnvalue (* (+ CurbIndex 1) (`self.CurbMeshLenth`)))
  (bind (_returnvalue_x _returnvalue_y _returnvalue_z) (`KismetMathLibrary.BreakVector` (+ (* (`SplineComponent.GetRightVectorAtDistanceAlongSpline` (`self.Spline`) _returnvalue "Local") (* (`self.CurbOffset`) -1.0)) (`SplineComponent.GetLocationAtDistanceAlongSpline` _spline _returnvalue "Local"))))
  (return (`KismetMathLibrary.MakeVector` _returnvalue_x _returnvalue_y (+ _returnvalue_z (`self.ZOffset`))) (`KismetMathLibrary.ClampVectorSize` (`SplineComponent.GetTangentAtDistanceAlongSpline` _spline _returnvalue "Local") 0.0 (`self.CurbMeshLenth`))))

(fn `MirrorCurbPosition`
  (params (CurbIndex :type Integer))
  (returns (StartingPositon :type "Vector Structure") (StartingTangent :type "Vector Structure"))
  (locals (NewLocalVar :type "Vector Structure"))
  (bind _spline (`self.Spline`))
  (bind _returnvalue (* CurbIndex (`self.CurbMeshLenth`)))
  (bind (_returnvalue_x _returnvalue_y _returnvalue_z) (`KismetMathLibrary.BreakVector` (+ (* (`SplineComponent.GetRightVectorAtDistanceAlongSpline` (`self.Spline`) _returnvalue "Local") (* (`self.CurbOffset`) -1.0)) (`SplineComponent.GetLocationAtDistanceAlongSpline` _spline _returnvalue "Local"))))
  (return (`KismetMathLibrary.MakeVector` _returnvalue_x _returnvalue_y (+ _returnvalue_z (`self.ZOffset`))) (`KismetMathLibrary.ClampVectorSize` (`SplineComponent.GetTangentAtDistanceAlongSpline` _spline _returnvalue "Local") 0.0 (`self.CurbMeshLenth`))))

(fn `StartingCurbPosition`
  (params (CurbIndex :type Integer))
  (returns (StartingPositon :type "Vector Structure") (StartingTangent :type "Vector Structure"))
  (locals (NewLocalVar :type "Vector Structure"))
  (return (0.0 0.0 0.0) (`KismetMathLibrary.ClampVectorSize` (`SplineComponent.GetTangentAtDistanceAlongSpline` (`self.Spline`) (* CurbIndex (`self.CurbMeshLenth`)) "Local") 0.0 (`self.CurbMeshLenth`))))

(fn `StartingRoadPosition`
  (params (RoadIndex :type Integer))
  (returns (StartingPositon :type "Vector Structure") (StartingTangent :type "Vector Structure"))
  (bind _spline (`self.Spline`))
  (bind _returnvalue (* RoadIndex (`self.RoadMeshLength`)))
  (return (`SplineComponent.GetLocationAtDistanceAlongSpline` _spline _returnvalue "Local") (`KismetMathLibrary.ClampVectorSize` (`SplineComponent.GetTangentAtDistanceAlongSpline` _spline _returnvalue "Local") 0.0 (`self.RoadMeshLength`))))

(fn `UserConstructionScript`
  (`|ExecutionSequence`
    (:`then_0`
      (for _index (range (+ (`KismetMathLibrary.FTrunc` (/ (`SplineComponent.GetSplineLength` (`self.Spline`)) (`self.RoadMeshLength`))) 1))
        (set `self.RoadIndex` _index)
        ; SpawnRoad
        (bind _returnvalue (`AddComponent|NODE_AddSplineMeshComponent-0`))
        (`StaticMeshComponent.SetStaticMesh` _returnvalue (`self.RoadStaticMesh`))
        (`SplineMeshComponent.SetForwardAxis` _returnvalue "X" true)
        (bind (_startingpositon _startingtangent) (`self.StartingRoadPosition` (`self.RoadIndex`)))
        (bind (_endingpositon _endingtangent) (`self.EndingRoadPosition` (`self.RoadIndex`)))
        (`SplineMeshComponent.SetStartAndEnd` _returnvalue _startingpositon _startingtangent _endingpositon _endingtangent true)))
    (:`then_1`
      (if (`self.Curbs`)
        (for _index_2 (range (+ (`KismetMathLibrary.FTrunc` (/ (`SplineComponent.GetSplineLength` (`self.Spline`)) (`self.CurbMeshLenth`))) 1))
          (set `self.CurbIndex` _index_2)
          (bind _returnvalue_2 (`AddComponent|NODE_AddSplineMeshComponent-1`))
          (`StaticMeshComponent.SetStaticMesh` _returnvalue_2 (`self.CurbStaticMesh`))
          (`SplineMeshComponent.SetForwardAxis` _returnvalue_2 "X" true)
          (bind (_startingpositon_2 _startingtangent_2) (`self.StartingCurbPosition` (`self.CurbIndex`)))
          (bind (_endingpositon_2 _endingtangent_2) (`self.EndingCurbPosition` (`self.CurbIndex`)))
          (`SplineMeshComponent.SetStartAndEnd` _returnvalue_2 _startingpositon_2 _startingtangent_2 _endingpositon_2 _endingtangent_2 true))))
    (:`then_2`
      (if (and (`self.Mirror`) (`self.Curbs`))
        (for _index_3 (range (+ (`KismetMathLibrary.FTrunc` (/ (`SplineComponent.GetSplineLength` (`self.Spline`)) (`self.CurbMeshLenth`))) 1))
          (set `self.CurbIndex` _index_3)
          (bind _returnvalue_3 (`AddComponent|NODE_AddSplineMeshComponent-2`))
          (`StaticMeshComponent.SetStaticMesh` _returnvalue_3 (`self.CurbStaticMesh`))
          (`SplineMeshComponent.SetForwardAxis` _returnvalue_3 "X" true)
          (bind (_startingpositon_3 _startingtangent_3) (`self.MirrorCurbPosition` (`self.CurbIndex`)))
          (bind (_endingpositon_3 _endingtangent_3) (`self.MirrorCurbPosionEnd` (`self.CurbIndex`)))
          (`SplineMeshComponent.SetStartAndEnd` _returnvalue_3 _startingpositon_3 _startingtangent_3 _endingpositon_3 _endingtangent_3 true))))))